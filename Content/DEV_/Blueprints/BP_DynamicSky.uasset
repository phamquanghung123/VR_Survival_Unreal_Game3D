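; Sky actor that sets sun, moon, atmosphere, fog, clouds and Sunny, Snowy or Rainy weather from TimeOfDay and a weather preset.
; The construction script applies everything through lights, a dynamic sky-sphere material, volumetric clouds and Niagara effects.
; Snow and rain force TimeOfDay to 11 and drive MPC_WeatherProperties for other materials.
; BeginPlay reapplies weather and optionally animates snow coverage with a timeline.
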(event `self.ReceiveBeginPlay`
  (bind (_shouldanimatesnowycoverageinruntime _fullsnowycoveragetime) (break `/Game/DEV_/DataAsset/S_SnowyWeatherSettings` (`self.SnowyWeatherSettings`)))
  (`self.HandleWeatherSettings`)
  (`self.GetCurrentWeatherType`
    (:`Snowy`
      (if _shouldanimatesnowycoverageinruntime
        (`KismetMaterialLibrary.SetScalarParameterValue` "/Game/DEV_/Materials/MaterialParameterCollection/MPC_WeatherProperties.MPC_WeatherProperties" "SnowyAmount")
        (`KismetSystemLibrary.Delay` 1.5)
        (`TimelineComponent.SetPlayRate` (`self.SnowyCoverageAnimationTimeline`) (/ 1.0 _fullsnowycoveragetime))
        (bind (_direction _normalizedfloat) (`Timeline|SnowyCoverageAnimationTimeline`)
          (:`Update`
            (`KismetMaterialLibrary.SetScalarParameterValue` "/Game/DEV_/Materials/MaterialParameterCollection/MPC_WeatherProperties.MPC_WeatherProperties" "SnowyAmount" _normalizedfloat)))))))

(fn `HandleCloudSetting`
  (`self.GetCurrentWeatherType`
    (:`Sunny`
      (switch `/Game/DEV_/ENUM/E_CloudMode` (`self.CurrentCloud`)
        (:`NewEnumerator0`
          (`self.Toggle2DCloud` false)
          (`self.ToggleVolumetricClouds` false))
        (:`NewEnumerator1`
          (`self.Toggle2DCloud` true)
          (`self.Set2DCloudSettingSunny`)
          (`self.ToggleVolumetricClouds` false))
        (:`NewEnumerator2`
          (`self.Toggle2DCloud` false)
          (`self.ToggleVolumetricClouds` true)
          (`self.SetVolumetricCloudSetting`))
        (:`NewEnumerator3`
          (`self.Toggle2DCloud` true)
          (`self.Set2DCloudSettingSunny`)
          (`self.ToggleVolumetricClouds` true)
          (`self.SetVolumetricCloudSetting`))))
    (:`Snowy`
      (`self.Toggle2DCloud` false)
      (`self.ToggleVolumetricClouds` false))
    (:`Rainy`
      (`self.Toggle2DCloud` true)
      (`self.Set2DCloudSettingRainy`)
      (`self.ToggleVolumetricClouds` false))))

(fn `HandleNightSetting`
  (if (`self.IsNightTime`)
    (`|ExecutionSequence`
      (:`then_0`
        (`LightComponent.SetIntensity` (`self.MoonDirectionalLight`) (`self.MoonLightIntensity`))
        (`LightComponent.SetLightColor` (`self.MoonDirectionalLight`) (`self.MoonLightColor`) true)
        (`DirectionalLightComponent.SetLightSourceAngle` (`self.MoonDirectionalLight`) (`self.MoonLightSourceAngle`))
        (`LightComponent.SetTemperature` (`self.MoonDirectionalLight`) (`self.MoonLightTemperature`)))
      (:`then_1`
        (`SkyAtmosphereComponent.SetRayleighScattering` (`self.SkyAtmosphere`) (`self.MoonLightRayleighScattering`))
        (`SkyAtmosphereComponent.SetMultiScatteringFactor` (`self.SkyAtmosphere`) (`self.NightTimeMultiScattering`)))
      (:`then_2`
        (`MaterialInstanceDynamic.SetScalarParameterValue` (`self.CreatedDymMISkySphere`) "IsStarVisibility" (`KismetMathLibrary.SelectFloat` 1.0 0.0 (`self.bShouldShowStars`)))
        (`MaterialInstanceDynamic.SetScalarParameterValue` (`self.CreatedDymMISkySphere`) "IsMoonVisibility" (`KismetMathLibrary.SelectFloat` 1.0 0.0 (`self.bShoulShowMoon`)))
        (`MaterialInstanceDynamic.SetVectorParameterValue` (`self.CreatedDymMISkySphere`) "MoonBasicSetting" (make `LinearColor` (/ (`self.MoonScale`) 10.0) (`self.MoonRotation`) (`self.MoonBrightness`) 1.0))
        (`MaterialInstanceDynamic.SetVectorParameterValue` (`self.CreatedDymMISkySphere`) "MoonTint" (`self.MoonTint`))))
    (else
      (`self.HandleWeatherSettings`)
      (`MaterialInstanceDynamic.SetScalarParameterValue` (`self.CreatedDymMISkySphere`) "IsStarVisibility" 0.0)
      (`MaterialInstanceDynamic.SetScalarParameterValue` (`self.CreatedDymMISkySphere`) "IsMoonVisibility" 0.0))))

(fn `HandleSunMoonRotation`
  ; Handling Sun Rotation Between draw and dusk
  (`SceneComponent.K2_SetWorldRotation` (`self.SunDirectionalLight`) (`KismetMathLibrary.MakeRotator` 0.0 (`KismetMathLibrary.MapRangeUnclamped` (`self.TimeOfDay`) (`self.DrawTime`) (`self.DuskTime`) 0.0 -180.0) (`self.SunMoonRotation`)) false false)
  ; Handle Moon after Sun Dusk
  (`SceneComponent.K2_SetWorldRotation` (`self.MoonDirectionalLight`) (`KismetMathLibrary.MakeRotator` 0.0 (`KismetMathLibrary.MapRangeUnclamped` (`self.TimeOfDay`) (+ (`self.DuskTime`) 0.3) 24.0 -180.0 -90.0) (`self.SunMoonRotation`)) false false)
  ; Handle Moon before Sun Draw
  (`SceneComponent.K2_SetWorldRotation` (`self.MoonDirectionalLight`) (`KismetMathLibrary.MakeRotator` 0.0 (`KismetMathLibrary.MapRangeUnclamped` (`self.TimeOfDay`) 0.0 (- (`self.DrawTime`) 0.3) -90.0) (`self.SunMoonRotation`)) false false))

(fn `HandleVisibility`
  (`SceneComponent.SetVisibility` (`self.SunDirectionalLight`) (`self.IsDayTime`) false)
  (`SceneComponent.SetVisibility` (`self.MoonDirectionalLight`) (`self.IsNightTime`) false))

(fn `HandleWeatherSettings`
  (`self.SetWeatherLightSettings`)
  (`self.GetCurrentWeatherType`
    (:`Sunny`
      (`self.ToggleSnowy` false)
      (`self.ToggleRain` false))
    (:`Snowy`
      (set `self.TimeOfDay` 11.0)
      (`self.ToggleSnowy` true)
      (`self.SetSnowyParticlesSetting`)
      (`self.ToggleRain` false))
    (:`Rainy`
      (set `self.TimeOfDay` 11.0)
      (`self.ToggleSnowy` false)
      (`self.ToggleRain` true)
      (`self.SetRainParticlesSettings`))))

(fn `InitSkySphereMaterial`
  (returns (IsDymMiSkySphereValid :type Boolean))
  (bind _returnvalue (`PrimitiveComponent.CreateDynamicMaterialInstance` (`self.SM_SkySphere`) 0 "/Game/DEV_/Materials/Sky/MI_DynamicSkySphere.MI_DynamicSkySphere" "None"))
  (bind _output_get (set `self.CreatedDymMISkySphere` _returnvalue))
  (return (`KismetSystemLibrary.IsValid` _output_get)))

(fn `SetWeatherLightSettings`
  (bind (_dirlightintensity _dirlightcolor _dirlightsourceangle _temperature) (break `/Game/DEV_/DataAsset/S_DirectionalLightSettings` (`/Game/DEV_/DataAsset/BP_WeatherDataAssetBase.DirectionalLightSettings` (`self.CurrentWeatherPreset`))))
  (bind (_multiscattering _rayleighscattering _miescatteringscale _mieabsorptionscale _mieanisotropy _aerialperspectiveviewdistancescale) (break `/Game/DEV_/DataAsset/S_SkyAtmosphereSettings` (`/Game/DEV_/DataAsset/BP_WeatherDataAssetBase.SkyAtmosphereSettings` (`self.CurrentWeatherPreset`))))
  (bind (_emissivecolor _extinctionscale) (break `/Game/DEV_/DataAsset/S_ExponentailHeightFogSettings` (`/Game/DEV_/DataAsset/BP_WeatherDataAssetBase.ExponentialHeightFogSettings` (`self.CurrentWeatherPreset`))))
  (if (`self.IsDayTime`)
    (`|ExecutionSequence`
      (:`then_0`
        (`LightComponent.SetIntensity` (`self.SunDirectionalLight`) _dirlightintensity)
        (`LightComponent.SetLightColor` (`self.SunDirectionalLight`) _dirlightcolor true)
        (`DirectionalLightComponent.SetLightSourceAngle` (`self.SunDirectionalLight`) _dirlightsourceangle)
        (`LightComponent.SetTemperature` (`self.SunDirectionalLight`) _temperature))
      (:`then_1`
        (`SkyLightComponent.SetIntensity` (`self.SkyLight`) (`.SkyLightIntensityScale_4_2A24DCA54F52473A4485D7A5771829E7` (break `/Game/DEV_/DataAsset/S_SkyLightSettings` (`/Game/DEV_/DataAsset/BP_WeatherDataAssetBase.SkyLightSettings` (`self.CurrentWeatherPreset`))))))
      (:`then_2`
        (`SkyAtmosphereComponent.SetMultiScatteringFactor` (`self.SkyAtmosphere`) _multiscattering)
        (`SkyAtmosphereComponent.SetRayleighScattering` (`self.SkyAtmosphere`) _rayleighscattering)
        (`SkyAtmosphereComponent.SetMieScatteringScale` (`self.SkyAtmosphere`) _miescatteringscale)
        (`SkyAtmosphereComponent.SetMieAbsorptionScale` (`self.SkyAtmosphere`) _mieabsorptionscale)
        (`SkyAtmosphereComponent.SetMieAnisotropy` (`self.SkyAtmosphere`) _mieanisotropy)
        (`SkyAtmosphereComponent.SetAerialPespectiveViewDistanceScale` (`self.SkyAtmosphere`) _aerialperspectiveviewdistancescale))
      (:`then_3`
        (`ExponentialHeightFogComponent.SetVolumetricFogEmissive` (`self.ExponentialHeightFog`) _emissivecolor)
        (`ExponentialHeightFogComponent.SetVolumetricFogExtinctionScale` (`self.ExponentialHeightFog`) _extinctionscale)))))

(fn `UserConstructionScript`
  (bind _isdymmiskyspherevalid (`self.InitSkySphereMaterial`))
  (if _isdymmiskyspherevalid
    (`|ExecutionSequence`
      (:`then_0`
        (`self.HandleWeatherSettings`))
      (:`then_1`
        (`self.HandleSunMoonRotation`))
      (:`then_2`
        (`self.HandleVisibility`))
      (:`then_3`
        (`self.HandleNightSetting`))
      (:`then_4`
        (`self.HandleCloudSetting`)))))